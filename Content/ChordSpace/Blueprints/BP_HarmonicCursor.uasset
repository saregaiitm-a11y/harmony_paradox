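; BP_HarmonicCursor is an actor that morphs a sound according to where a grabbing hand sits between two nodes, NodeA and NodeB.
; While active, Tick projects the hand's world position onto the node segment, clamps it to a normalized BlendValue and feeds that to the audio's Morph parameter.
; StartAudio activates it and starts playback; FadeAndDespawn deactivates it, stops the audio and destroys the actor after a short delay.
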(event `self.ReceiveTick`
  (params (DeltaSeconds :type "Float (single-precision)"))
  (bind _grabbing_hand (`self.Grabbing Hand`))
  (bind _nodea (`self.NodeA`))
  (bind _returnvalue (- (`self.NodeB`) _nodea))
  (bind _returnvalue_2 (`KismetMathLibrary.FClamp` (/ (`KismetMathLibrary.Dot_VectorVector` (- (`SceneComponent.K2_GetComponentLocation` _grabbing_hand) _nodea) _returnvalue) (`KismetMathLibrary.Dot_VectorVector` _returnvalue _returnvalue))))
  (if (`self.isActive`)
    (if (`KismetSystemLibrary.IsValid` _grabbing_hand)
      (set `self.BlendValue` _returnvalue_2)
      (`AudioParameterControllerInterface.SetFloatParameter` (`self.Audio`) "Morph" _returnvalue_2))))

(event `self.ReceiveBeginPlay`
  (set `self.isActive` false))

(event `FadeAndDespawn`
  ; FadeAndDespawn
  (set `self.isActive` false)
  (`AudioComponent.Stop` (`self.Audio`))
  (`KismetSystemLibrary.Delay` 1.6)
  (`self.K2_DestroyActor`))

(fn `StartAudio`
  (set `self.isActive` true)
  (`AudioComponent.Play` (`self.Audio`) 0.0))

(fn `UserConstructionScript`)