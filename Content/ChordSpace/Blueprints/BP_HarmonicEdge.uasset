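; BP_HarmonicEdge is a ChordSpace edge between two spheres that lets an XR player spawn a sound-playing harmonic cursor on it.
; Collision overlaps record the touching component as the overlapping hand whenever the player pawn is a BP_XRPawn.
; TrySpawnCursor creates one BP_HarmonicCursor at that hand, passes it both spheres as nodes and starts its audio, leaving attachment code unconnected.
; TryDespawnCursor fades out and clears the active cursor.
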(event `self.EdgeCollision.OnComponentBeginOverlap`
  (params (OverlappedComponent :type "PrimitiveComponent Object Reference") (OtherActor :type "Actor Object Reference") (OtherComp :type "PrimitiveComponent Object Reference") (OtherBodyIndex :type Integer) (bFromSweep :type Boolean) (SweepResult :type "HitResult Structure (by ref)"))
  ; Start Overlap
  (cast `/Game/XRFramework/Blueprints/BP_XRPawn` (`GameplayStatics.GetPlayerPawn` 0))
  (set `self.IsHandOverlapping` true)
  (set `self.OverlappingHand` OtherComp))

(event `self.EdgeCollision.OnComponentEndOverlap`
  (params (OverlappedComponent :type "PrimitiveComponent Object Reference") (OtherActor :type "Actor Object Reference") (OtherComp :type "PrimitiveComponent Object Reference") (OtherBodyIndex :type Integer))
  ; End Overlap
  (cast `/Game/XRFramework/Blueprints/BP_XRPawn` (`GameplayStatics.GetPlayerPawn` 0))
  (set `self.IsHandOverlapping` false)
  (set `self.OverlappingHand` null))

(event `TryDespawnCursor`
  (bind _activecursor (`self.ActiveCursor`))
  ; TryDespawnCursor
  (if (`KismetSystemLibrary.IsValid` _activecursor)
    (`/Game/ChordSpace/Blueprints/BP_HarmonicCursor.FadeAndDespawn` _activecursor)
    (set `self.ActiveCursor` null)))

(event `TrySpawnCursor`
  ; TrySpawnCursor
  (if (and (`self.IsHandOverlapping`) (not (`KismetSystemLibrary.IsValid` (`self.ActiveCursor`))))
    (bind _returnvalue (`|SpawnActorFromClass` "/Game/ChordSpace/Blueprints/BP_HarmonicCursor.BP_HarmonicCursor_C" (`KismetMathLibrary.MakeTransform` (`SceneComponent.K2_GetComponentLocation` (`self.OverlappingHand`))) "AlwaysSpawn" "MultiplyWithRoot" null null))
    (set `self.ActiveCursor` _returnvalue)
    (set `/Game/ChordSpace/Blueprints/BP_HarmonicCursor.NodeA` (`self.SphereA`) _returnvalue)
    (set `/Game/ChordSpace/Blueprints/BP_HarmonicCursor.NodeB` (`self.SphereB`) _returnvalue)
    (set `self.GrabbingHand` _returnvalue)
    (`/Game/ChordSpace/Blueprints/BP_HarmonicCursor.StartAudio` (`self.ActiveCursor`))))

(fn `UserConstructionScript`)