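; BP_HarmonyCore is an actor that bobs up and down in place and detects overlaps with its sphere collision.
; BeginPlay stores the starting height, and Tick offsets Z from it with a sine of game time, without sweeping.
; The sphere overlap event only prints a debug message, with no further gameplay effect in this Blueprint.
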(event `self.ReceiveBeginPlay`
  (bind _output_get (set `self.BaseZ` (.z (`self.K2_GetActorLocation`)))))

(event `self.ReceiveTick`
  (params (DeltaSeconds :type "Float (single-precision)"))
  (`self.K2_SetActorLocation` (`KismetMathLibrary.MakeVector` (.x (`self.K2_GetActorLocation`)) (.y (`self.K2_GetActorLocation`)) (+ (* (`KismetMathLibrary.Sin` (`KismetSystemLibrary.GetGameTimeInSeconds`)) 20.0) (stale `self.ReceiveBeginPlay` _output_get)))))

(event `self.SphereCollision.OnComponentBeginOverlap`
  (params (OverlappedComponent :type "PrimitiveComponent Object Reference") (OtherActor :type "Actor Object Reference") (OtherComp :type "PrimitiveComponent Object Reference") (OtherBodyIndex :type Integer) (bFromSweep :type Boolean) (SweepResult :type "HitResult Structure (by ref)"))
  (`KismetSystemLibrary.PrintString` "C_playing!!!" true true (struct :`G` 0.66 :`B` 1.0 :`A` 1.0) 10.0))

(fn `UserConstructionScript`)